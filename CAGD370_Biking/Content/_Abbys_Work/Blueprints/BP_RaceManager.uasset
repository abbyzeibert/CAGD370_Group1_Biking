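; BP_RaceManager runs a bike time trial and doubles as the finish-line trigger, handling countdown, start, end and restart.
; A Delay-driven loop counts race time in tenths of a second into a Timecode, while Tick derives speed from bike velocity.
; Finishing inserts the time into the current level's GameInstance list, longest first, saves it to that level's slot and opens the main menu.
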(event Custom|ResetRace
  ;[0 1 0 0.5] Add as a Pause Menu option, for now hold R for 3 seconds
  (CallFunction|RestartRace)
  (Utilities|RaceCountdown)
  (CallFunction|StartRace)
  (Utilities|RunTimer))

(event EventBeginPlay
  ;[0 1 0 0.5] Initilizes references and starts race
  (Utilities|FlowControl|Delay 0.1)
  (bind _asbp_game_instance (Utilities|Casting|CastToBP_GameInstance (Game|GetGameInstance)))
  (Variables|Default|SetGameInstance _asbp_game_instance)
  (bind _returnvalue (Actor|GetActorOfClass "/Game/_Abbys_Work/Blueprints/SaveObjects/BP_Score.BP_Score_C"))
  (Variables|Default|SetCurScore _returnvalue)
  (bind _returnvalue_2 (Actor|GetActorOfClass "/Game/_Abbys_Work/Blueprints/BP_Bike.BP_Bike_C"))
  (bind _output_get (Variables|Default|SetBike _returnvalue_2))
  (bind _output_get_2 (Variables|Default|SetStartPoint (Transformation|GetActorTransform _output_get)))
  (Variables|Default|SetRespawnPoint _output_get_2)
  (Utilities|RaceCountdown)
  (CallFunction|StartRace)
  (Utilities|RunTimer))

(event Collision|EventActorBeginOverlap
  (params (OtherActor :type Actor%20Object%20Reference))
  ;[0 1 0 0.5] Ends race when player hits finish line
  (Utilities|Casting|CastToBP_Bike OtherActor)
  (CallFunction|EndRace)
  (Utilities|AddScoretoList
    (:Out
      (SaveGame|SaveGametoSlot (Variables|Default|GetCurSave) (Variables|Default|GetCurSlotName))
      (Utilities|FlowControl|Delay 3.0)
      (Game|OpenLevel(byObjectReference) "/Game/_Tophers_Work/_Levels/LV_MainMenu.LV_MainMenu"))))

(event EventTick
  (params (DeltaSeconds :type Float%20%28single-precision%29))
  (bind _bike (Variables|Default|GetBike))
  ;[0 1 0 0.5] Creates speed from falling and forward velocity
  (if (Variables|Default|GetRaceActive)
    (Variables|Default|SetSpeed (Math|Float|Absolute(Float) (/ (+ (Variables|/Game/_Abbys_Work/Blueprints/BP_Bike.BP_Bike_C|GetVelocity _bike) (Math|Float|Absolute(Float) (Variables|/Game/_Abbys_Work/Blueprints/BP_Bike.BP_Bike_C|GetFallingVelocity _bike))) 1e+01)))))

(fn ConstructionScript)

(fn StartRace
  (Default|StartRace (Variables|Default|GetBike))
  (Variables|Default|SetRaceActive true))

(fn EndRace
  (Default|EndRace (Variables|Default|GetBike))
  (Variables|/Game/_Abbys_Work/Blueprints/SaveObjects/BP_Score.BP_Score_C|SetTime (Variables|Default|GetCurScore) (Variables|Default|GetTimer))
  (Variables|Default|SetRaceActive false))

(fn Respawn
  (bind _bike (Variables|Default|GetBike))
  (bind _output_get (Variables|/Game/_Abbys_Work/Blueprints/BP_Bike.BP_Bike_C|SetVelocity _bike 0.0))
  (Variables|/Game/_Abbys_Work/Blueprints/BP_Bike.BP_Bike_C|SetFallingVelocity _bike _output_get)
  (Transformation|SetActorTransform _bike (Variables|Default|GetRespawnPoint)))

(fn RestartRace
  (CallFunction|EndRace)
  (Variables|Default|SetMiliseconds 0)
  (Variables|Default|SetSeconds 0)
  (Variables|Default|SetMinutes 0)
  (Variables|Default|SetRespawnPoint (Variables|Default|GetStartPoint))
  (Variables|Default|SetCountdown 3)
  (CallFunction|Respawn))