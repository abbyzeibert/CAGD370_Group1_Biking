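; Player-controlled trick bike for races, with pedaling, braking, turning, jumping and airborne spins and flips.
; Tick drives kinematic movement without physics, using traces to follow slopes, bounce off walls and prevent floor clipping, with RaceManager respawn as fallback.
; Timelines animate tricks, wobbles, crashes and landing camera shake, while the spring arm follows slope and fall.
; Landings judge trick completion to bank diminishing-repeat scores or trigger graded fails.
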(event Custom|ShakeCamera
  ;[0 1 0 0.5] Camera shake
  (Development|PrintString "Shaking cam")
  (Transformation|SetWorldRotation (Variables|Default|GetSpringArm) (Math|Rotator|MakeRotator 0.0 (Variables|Default|GetDefaultCamRot) (.yaw (Transformation|GetActorRotation))) false false)
  (bind _springarmrotation (Timeline|CameraShake PlayFromStart)
    (:Update
      (Transformation|AddLocalRotation (Variables|Default|GetSpringArm) (Math|Rotator|MakeRotator 0.0 (* _springarmrotation (Math|Float|Clamp(Float) (/ (Math|Float|Absolute(Float) (Variables|Default|GetPrevFallingVelocity)) 5e+01) 0.0 3e+01)) 0.0) false false))
    (:Finished
      (Variables|Default|SetIsShaking false))))

(event Custom|Crash
  ;[0 1 0 0.5] Major Crash timeline
  (Development|PrintString "Starting crash")
  (Transformation|SetRelativeLocation (Variables|Default|GetFailMesh) (Math|Vector|MakeVector 0.0 0.0 25.0) false false)
  (bind _spinintensity (Timeline|CrashFlip PlayFromStart)
    (:Update
      (Transformation|SetRelativeRotation (Variables|Default|GetBikeMesh) (Math|Rotator|MakeRotator 0.0 _spinintensity 0.0) false false))
    (:Finished
      (Variables|Default|SetIsCrashing false)
      (Transformation|SetRelativeLocation (Variables|Default|GetFailMesh) (Math|Vector|MakeVector 0.0 0.0 0.0) false false))))

(event Custom|StopTrick
  (Utilities|FlowControl|Sequence
    (:then_0
      ;[0 1 0 0.5] Spins bike right while in the air
      (bind (_direction _trickcompletion _bikerotation) (Timeline|RightSpin Stop)
        (:Update
          (Variables|Default|SetTrickCompletion _trickcompletion)
          (Transformation|SetRelativeRotation (Variables|Default|GetFailMesh) (Math|Rotator|MakeRotator 0.0 0.0 _bikerotation) false false))
        (:Finished
          (Variables|Default|SetTrickCompletion 0.0))))
    (:then_1
      ;[0 1 0 0.5] Spins bike left while in the air
      (bind (_direction_2 _trickcompletion_2 _bikerotation_2) (Timeline|LeftSpin Stop)
        (:Update
          (Variables|Default|SetTrickCompletion _trickcompletion_2)
          (Transformation|SetRelativeRotation (Variables|Default|GetFailMesh) (Math|Rotator|MakeRotator 0.0 0.0 _bikerotation_2) false false))
        (:Finished
          (Variables|Default|SetTrickCompletion 0.0))))
    (:then_2
      ;[0 1 0 0.5] Frontflip
      (bind (_direction_3 _trickcompletion_3 _bikerotation_3) (Timeline|Frontflip Stop)
        (:Update
          (Variables|Default|SetTrickCompletion _trickcompletion_3)
          (Transformation|SetRelativeRotation (Variables|Default|GetFailMesh) (Math|Rotator|MakeRotator 0.0 _bikerotation_3 0.0) false false))
        (:Finished
          (Variables|Default|SetTrickCompletion 0.0))))
    (:then_3
      ;[0 1 0 0.5] Backflip
      (bind (_direction_4 _trickcompletion_4 _bikerotation_4) (Timeline|Backflip Stop)
        (:Update
          (Variables|Default|SetTrickCompletion _trickcompletion_4)
          (Transformation|SetRelativeRotation (Variables|Default|GetFailMesh) (Math|Rotator|MakeRotator 0.0 _bikerotation_4 0.0) false false))
        (:Finished
          (Variables|Default|SetTrickCompletion 0.0))))
    (:then_4
      (Utilities|LandfromTrick))))

(event Custom|Wobble
  (params (MinorFail :type Boolean))
  (Development|PrintString "Starting wobble")
  (bind _wobbleamount (Timeline|TurnWobble PlayFromStart)
    (:Update
      (if MinorFail
        (Variables|Default|SetWobbleMultiplier 2.0)
        (else
          (Variables|Default|SetWobbleMultiplier 4.0)))
      (Variables|Default|SetWobbleAmt (* _wobbleamount (Variables|Default|GetWobbleMultiplier))))
    (:Finished
      (Variables|Default|SetWobbleAmt 0.0))))

(event Custom|StartRace
  ;[0 1 0 0.5] Race controls
  (Variables|Default|SetIsActive true)
  (Development|PrintString "Race Started!"))

(event Custom|EndRace
  ;[0 1 0 0.5] Race controls
  (Variables|Default|SetIsActive false)
  (Development|PrintString "Race Ended!"))

(event Input|EnhancedActionEvents|EnhancedInputActionIA_Pedal
  (params (ActionValue :type Boolean) (ElapsedSeconds :type Float%20%28double-precision%29) (TriggeredSeconds :type Float%20%28double-precision%29) (InputAction :type Input%20Action%20Object%20Reference :default "/Game/_Abbys_Work/Blueprints/Input/IA_Pedal.IA_Pedal"))
  ;[0 1 0 0.5] When player presses forward, adds to Velocity until max is reached
  (:Triggered
    (if (not (Variables|Default|GetIsCrashing))
      (Variables|Default|SetIsPedaling true)))
  (:Completed
    (Variables|Default|SetIsPedaling false)))

(event Input|EnhancedActionEvents|EnhancedInputActionIA_Brake
  (params (ActionValue :type Boolean) (ElapsedSeconds :type Float%20%28double-precision%29) (TriggeredSeconds :type Float%20%28double-precision%29) (InputAction :type Input%20Action%20Object%20Reference :default "/Game/_Abbys_Work/Blueprints/Input/IA_Brake.IA_Brake"))
  ;[0 1 0 0.5] Increases friction while braking
  (:Triggered
    (Variables|Default|SetFriction (Variables|Default|GetBrakingFriction))
    (Variables|Default|SetIsBraking true))
  (:Completed
    (if (not (Variables|Default|GetIsCrashing))
      (Variables|Default|SetFriction (Variables|Default|GetStandardFriction))
      (Variables|Default|SetIsBraking false))))

(event Input|EnhancedActionEvents|EnhancedInputActionIA_LeftSpin
  (params (ActionValue :type Boolean) (ElapsedSeconds :type Float%20%28double-precision%29) (TriggeredSeconds :type Float%20%28double-precision%29) (InputAction :type Input%20Action%20Object%20Reference :default "/Game/_Abbys_Work/Blueprints/Input/IA_LeftSpin.IA_LeftSpin"))
  ;[0 1 0 0.5] Spins bike left while in the air
  (if (not (Variables|Default|GetIsCrashing))
    (if (Variables|Default|GetIsActive)
      (if (not (Variables|Default|GetOnGround))
        (if (== (Variables|Default|GetTrickCompletion) 0.0)
          (Utilities|DoCurTrickScore "Left Spin" 250
            (:true
              (bind (_direction _trickcompletion _bikerotation) (Timeline|LeftSpin PlayFromStart)
                (:Update
                  (Variables|Default|SetTrickCompletion _trickcompletion)
                  (Transformation|SetRelativeRotation (Variables|Default|GetFailMesh) (Math|Rotator|MakeRotator 0.0 0.0 _bikerotation) false false))
                (:Finished
                  (Variables|Default|SetTrickCompletion 0.0))))))))))

(event Input|EnhancedActionEvents|EnhancedInputActionIA_Backflip
  (params (ActionValue :type Boolean) (ElapsedSeconds :type Float%20%28double-precision%29) (TriggeredSeconds :type Float%20%28double-precision%29) (InputAction :type Input%20Action%20Object%20Reference :default "/Game/_Abbys_Work/Blueprints/Input/IA_Backflip.IA_Backflip"))
  ;[0 1 0 0.5] Backflip
  (if (not (Variables|Default|GetIsCrashing))
    (if (Variables|Default|GetIsActive)
      (if (not (Variables|Default|GetOnGround))
        (if (== (Variables|Default|GetTrickCompletion) 0.0)
          (Utilities|DoCurTrickScore "Backflip" 500
            (:true
              (bind (_direction _trickcompletion _bikerotation) (Timeline|Backflip PlayFromStart)
                (:Update
                  (Variables|Default|SetTrickCompletion _trickcompletion)
                  (Transformation|SetRelativeRotation (Variables|Default|GetFailMesh) (Math|Rotator|MakeRotator 0.0 _bikerotation 0.0) false false))
                (:Finished
                  (Variables|Default|SetTrickCompletion 0.0))))))))))

(event Input|EnhancedActionEvents|EnhancedInputActionIA_Turn
  (params (ActionValue :type Float%20%28double-precision%29) (ElapsedSeconds :type Float%20%28double-precision%29) (TriggeredSeconds :type Float%20%28double-precision%29) (InputAction :type Input%20Action%20Object%20Reference :default "/Game/_Abbys_Work/Blueprints/Input/IA_Turn.IA_Turn"))
  ;[0 1 0 0.5] Activates & deactivates turning
  (:Triggered
    (if (not (Variables|Default|GetIsCrashing))
      (if (Variables|Default|GetOnGround)
        (Variables|Default|SetTurnDir ActionValue)
        (else
          (Variables|Default|SetTurnDir 0.0 :!label _label)))))
  (:Completed
    (goto _label)))

(event Input|EnhancedActionEvents|EnhancedInputActionIA_Jump
  (params (ActionValue :type Boolean) (ElapsedSeconds :type Float%20%28double-precision%29) (TriggeredSeconds :type Float%20%28double-precision%29) (InputAction :type Input%20Action%20Object%20Reference :default "/Game/_Abbys_Work/Blueprints/Input/IA_Jump.IA_Jump"))
  (if (not (Variables|Default|GetIsCrashing))
    (if (Variables|Default|GetIsActive)
      (if (Variables|Default|GetOnGround)
        (CallFunction|Jump)))))

(event Input|EnhancedActionEvents|EnhancedInputActionIA_Restart
  (params (ActionValue :type Boolean) (ElapsedSeconds :type Float%20%28double-precision%29) (TriggeredSeconds :type Float%20%28double-precision%29) (InputAction :type Input%20Action%20Object%20Reference :default "/Game/_Abbys_Work/Blueprints/Input/IA_Restart.IA_Restart"))
  ;[0 1 0 0.5] Race controls
  (Default|ResetRace (Variables|Default|GetRaceManager)))

(event Input|EnhancedActionEvents|EnhancedInputActionIA_RightSpin
  (params (ActionValue :type Boolean) (ElapsedSeconds :type Float%20%28double-precision%29) (TriggeredSeconds :type Float%20%28double-precision%29) (InputAction :type Input%20Action%20Object%20Reference :default "/Game/_Abbys_Work/Blueprints/Input/IA_RightSpin.IA_RightSpin"))
  ;[0 1 0 0.5] Spins bike right while in the air
  (if (not (Variables|Default|GetIsCrashing))
    (if (Variables|Default|GetIsActive)
      (if (not (Variables|Default|GetOnGround))
        (if (== (Variables|Default|GetTrickCompletion) 0.0)
          (Utilities|DoCurTrickScore "Right Spin" 250
            (:true
              (bind (_direction _trickcompletion _bikerotation) (Timeline|RightSpin PlayFromStart)
                (:Update
                  (Variables|Default|SetTrickCompletion _trickcompletion)
                  (Transformation|SetRelativeRotation (Variables|Default|GetFailMesh) (Math|Rotator|MakeRotator 0.0 0.0 _bikerotation) false false))
                (:Finished
                  (Variables|Default|SetTrickCompletion 0.0))))))))))

(event Input|EnhancedActionEvents|EnhancedInputActionIA_Frontflip
  (params (ActionValue :type Boolean) (ElapsedSeconds :type Float%20%28double-precision%29) (TriggeredSeconds :type Float%20%28double-precision%29) (InputAction :type Input%20Action%20Object%20Reference :default "/Game/_Abbys_Work/Blueprints/Input/IA_Frontflip.IA_Frontflip"))
  ;[0 1 0 0.5] Frontflip
  (if (not (Variables|Default|GetIsCrashing))
    (if (Variables|Default|GetIsActive)
      (if (not (Variables|Default|GetOnGround))
        (if (== (Variables|Default|GetTrickCompletion) 0.0)
          (Utilities|DoCurTrickScore "Frontflip" 500
            (:true
              (bind (_direction _trickcompletion _bikerotation) (Timeline|Frontflip PlayFromStart)
                (:Update
                  (Variables|Default|SetTrickCompletion _trickcompletion)
                  (Transformation|SetRelativeRotation (Variables|Default|GetFailMesh) (Math|Rotator|MakeRotator 0.0 _bikerotation 0.0) false false))
                (:Finished
                  (Variables|Default|SetTrickCompletion 0.0))))))))))

(event EventBeginPlay
  (bind _returnvalue (Game|GetPlayerController 0))
  (Utilities|FlowControl|Delay 0.1)
  ;[0 1 0 0.5] Setting up input mapping
  (bind _asbp_player_controller (Utilities|Casting|CastToBP_PlayerController _returnvalue))
  (Input|AddMappingContext (PlayerController|LocalPlayerSubsystems|GetEnhancedInputLocalPlayerSubsystem _asbp_player_controller) "/Game/_Abbys_Work/Blueprints/Input/IMC_BikeControls.IMC_BikeControls" 0 "(bIgnoreAllPressedKeysUntilRelease=True,bForceImmediately=False,bNotifyUserSettings=False)")
  (Input|SetInputModeGameOnly _returnvalue false)
  (bind _returnvalue_2 (Actor|GetActorOfClass "/Game/_Abbys_Work/Blueprints/BP_RaceManager.BP_RaceManager_C"))
  (Variables|Default|SetRaceManager _returnvalue_2))

(event EventTick
  (params (DeltaSeconds :type Float%20%28single-precision%29))
  (bind _returnvalue (Transformation|GetActorForwardVector))
  (bind _returnvalue_2 (Math|Trig|Sin(Degrees) (.z _returnvalue)))
  (bind _output_get (Variables|Default|SetDelta%20Seconds DeltaSeconds))
  (if (Variables|Default|GetIsActive)
    (if (Variables|Default|GetOnGround)
      (if (Variables|Default|GetIsPedaling)
        (Variables|Default|SetVelocity (Math|Float|Clamp(Float) (+ (* (Variables|Default|GetAcceleration) (Variables|Default|GetDelta%20Seconds)) (Math|Float|Clamp(Float) (- (Variables|Default|GetVelocity) (* (Variables|Default|GetFriction) (Variables|Default|GetDelta%20Seconds))) 0.0 (Variables|Default|GetMaxVelocity))) -1e+02 (Variables|Default|GetMaxVelocity)))
        (else
          (Variables|Default|SetVelocity (Math|Float|Clamp(Float) (- (Variables|Default|GetVelocity) (* (Variables|Default|GetFriction) (Variables|Default|GetDelta%20Seconds))) 0.0 (Variables|Default|GetMaxVelocity))))))
    ;[0 1 0 0.5] Angles bike based on slope and changes velocity from slope
    (CallFunction|TurnAlongSlope)
    (Variables|Default|SetBikeAngle _returnvalue_2)
    ;[0 1 0 0.5] Moves bike in forward direction with given velocity
    (Variables|Default|SetVelocity (- (Variables|Default|GetVelocity) (* _returnvalue_2 (Variables|Default|GetHillSpeedMultiplier) (Variables|Default|GetDelta%20Seconds))))
    (Transformation|AddActorWorldOffset (* (Transformation|GetActorForwardVector) (Variables|Default|GetVelocity) _output_get))
    ;[0 1 0 0.5] Turns bike based on turn direction and speed
    (Class|Actor|AddActorWorldRotation (Math|Rotator|MakeRotator 0.0 0.0 (* (+ (Variables|Default|GetTurnDir) (Variables|Default|GetWobbleAmt)) (Variables|Default|GetTurnSpeed) (Variables|Default|GetDelta%20Seconds))))
    (CallFunction|BounceOffWalls)
    (CallFunction|AngleCameratoSlope)
    (CallFunction|PreventFloorClipping)))

(fn ConstructionScript)

(fn TurnAlongSlope
  (bind _returnvalue (Transformation|GetActorLocation))
  (bind _returnvalue_2 (Transformation|GetActorLocation))
  (bind (_outhit _returnvalue_3) (Collision|LineTraceForObjects _returnvalue_2 (+ _returnvalue_2 (* (Math|Vector|GetUpVector "0, 0, 0") (Variables|Default|GetDownCastLength))) (Variables|Default|GetObject%20Types) false 0 "None"))
  (if _returnvalue_3
    (if (Variables|Default|GetOnGround)
      _
      (else
        (Utilities|HitGround)))
    (Transformation|SetActorLocation (Math|Vector|MakeVector (.x _returnvalue) (.y _returnvalue) (+ (Variables|Default|GetBikeHeight) (.z (.ImpactPoint (Collision|BreakHitResult _outhit))))) false false)
    (Transformation|SetActorRotation (Math|Rotator|MakeRotator (.roll (Math|Rotator|MakeRotfromXZ (Transformation|GetActorForwardVector) (.ImpactNormal (Collision|BreakHitResult _outhit)))) (.pitch (Class|KismetMathLibrary|MakeRotfromYZ (Transformation|GetActorRightVector) (.ImpactNormal (Collision|BreakHitResult _outhit)))) (.yaw (Transformation|GetActorRotation))))
    (else
      (if (Variables|Default|GetOnGround)
        (Variables|Default|SetOnGround false)
        (Variables|Default|SetFallingVelocity 0.0)
        (Variables|Default|SetDownCastLength -3e+01))
      (CallFunction|Fall)))
  (return))

(fn Jump
  (Transformation|AddActorWorldOffset (Math|Vector|MakeVector 0.0 0.0 1e+01))
  (Variables|Default|SetOnGround false)
  (Variables|Default|SetDownCastLength -3e+01)
  (Variables|Default|SetFallingVelocity (Variables|Default|GetJumpForce))
  (Transformation|SetActorRotation (Math|Rotator|MakeRotator 0.0 0.0 (.yaw (Transformation|GetActorRotation)))))

(fn Fall
  (bind _delta_seconds (Variables|Default|GetDelta%20Seconds))
  (bind _output_get (Variables|Default|SetFallingVelocity (- (Variables|Default|GetFallingVelocity) (* (Variables|Default|GetGravity) _delta_seconds))))
  (Transformation|AddActorLocalOffset (Math|Vector|MakeVector 0.0 0.0 (* _output_get _delta_seconds)) false false))

(fn AngleCameratoSlope
  (bind _returnvalue (Transformation|GetActorRotation))
  (bind _springarm (Variables|Default|GetSpringArm))
  (bind _fallingvelocity (Variables|Default|GetFallingVelocity))
  (bind _defaultspringspeed (Variables|Default|GetDefaultSpringSpeed))
  (bind _returnvalue_2 (Class|SpringArmComponent|GetTargetRotation _springarm))
  (if (Variables|Default|GetOnGround)
    (Variables|/Script/Engine.SpringArmComponent|SetSocketOffset (Variables|Default|GetSpringArm) (Math|Vector|MakeVector (- (Variables|Default|GetDefaultSpringSpeed) (/ (Variables|Default|GetVelocity) 1e+01)) 0.0 (Math|Float|Lerp (.z (Variables|/Script/Engine.SpringArmComponent|GetSocketOffset (Variables|Default|GetSpringArm))) (- (Variables|Default|GetDefaultSpringPos) (* (Variables|Default|GetBikeAngle) 7.5e+03)) 0.15)))
    (if (not (Variables|Default|GetIsShaking))
      (Transformation|SetWorldRotation (Variables|Default|GetSpringArm) (Math|Rotator|MakeRotator 0.0 (Math|Float|Clamp(Float) (+ (Variables|Default|GetDefaultCamRot) (* (Variables|Default|GetBikeAngle) 1875.0)) -2e+01 2e+01) (.yaw _returnvalue)) false false))
    (elif (> (.pitch _returnvalue_2) (LocalVariables|GetMaxFallingAngle))
      (Transformation|AddLocalRotation _springarm (Math|Rotator|MakeRotator 0.0 (* (LocalVariables|GetFallingAcceleration) (Variables|Default|GetDelta%20Seconds) -1.0) 0.0) false false)
      (Transformation|SetWorldRotation _springarm (Math|Rotator|MakeRotator 0.0 (.pitch _returnvalue_2) (.yaw _returnvalue)) false false)
      (Variables|/Script/Engine.SpringArmComponent|SetSocketOffset _springarm (Math|Vector|MakeVector (Math|Float|Clamp(Float) (+ _fallingvelocity _defaultspringspeed) -6e+02 _defaultspringspeed) 0.0 (Math|Float|Clamp(Float) (- (.z (Variables|/Script/Engine.SpringArmComponent|GetSocketOffset _springarm)) (/ _fallingvelocity 2e+01)) (.z (Variables|/Script/Engine.SpringArmComponent|GetSocketOffset _springarm)) 1e+03))))))

(fn BounceOffWalls
  (bind _returnvalue (Transformation|GetActorForwardVector))
  (bind _returnvalue_2 (Transformation|GetActorForwardVector))
  (bind _returnvalue_3 (Transformation|GetActorLocation))
  (bind _returnvalue_4 (* _returnvalue_2 5e+01))
  ;[0 1 0 0.5] Capsule trace size of bike to check for walls
  (bind (_outhit _returnvalue_5) (Class|KismetSystemLibrary|CapsuleTraceSingleforObjects (+ _returnvalue_4 _returnvalue_3) (- _returnvalue_3 _returnvalue_4) 5.0 0.0 (Variables|Default|GetObject%20Types) false 0 "None" true))
  ;[0 1 0 0.5] Find the angle of the wall hit, if it is close to straight up, it's a wall
  (if _returnvalue_5
    ;[0 1 0 0.5] If going slowly, stop the bike
    (if (> (Variables|Default|GetVelocity) 3e+02)
      (if (and (<= (* (Math|Trig|Sin(Degrees) (.Z (Math|Vector|BreakVector (.ImpactNormal (Collision|BreakHitResult _outhit))))) 1e+02) 1.0) (>= (* (Math|Trig|Sin(Degrees) (.Z (Math|Vector|BreakVector (.ImpactNormal (Collision|BreakHitResult _outhit))))) 1e+02) -1.0))
        (if (> (Math|Float|Absolute(Float) (Class|KismetMathLibrary|VectorCosineAngle2D (.ImpactNormal (Collision|BreakHitResult _outhit)) _returnvalue)) 0.85)
          ;[0 1 0 0.5] At steep angle, bounce backwards from wall
          (Transformation|AddActorWorldOffset (* (.ImpactNormal (Collision|BreakHitResult _outhit)) (Variables|Default|GetMoveAwayFromWall)))
          (CallFunction|Jump)
          (Variables|Default|SetVelocity -3e+02)
          (else
            ;[0 1 0 0.5] At shallow angle, reflect off wall and lose some speed
            (Transformation|AddActorWorldOffset (* (.ImpactNormal (Collision|BreakHitResult _outhit)) (Variables|Default|GetMoveAwayFromWall)))
            (Transformation|SetActorRotation (Math|Conversions|RotationFromXVector (Math|Vector|GetReflectionVector _returnvalue (.ImpactNormal (Collision|BreakHitResult _outhit)))))
            (Variables|Default|SetVelocity (* (Variables|Default|GetVelocity) (- 1.0 (Math|Float|Absolute(Float) (Class|KismetMathLibrary|VectorCosineAngle2D (.ImpactNormal (Collision|BreakHitResult _outhit)) _returnvalue)))))
            (Development|PrintString "Bonk!"))))
      (else
        (Variables|Default|SetVelocity 0.0)))))

(fn PreventFloorClipping
  (bind _returnvalue (Transformation|GetActorLocation))
  (bind _returnvalue_2 (Transformation|GetActorLocation))
  (if (not (Variables|Default|GetOnGround))
    (bind _returnvalue_3 (Collision|LineTraceForObjects _returnvalue_2 (+ _returnvalue_2 (* (Math|Vector|GetUpVector "0, 0, 0") (* (Variables|Default|GetFindGroundLength) -1.0))) (Variables|Default|GetFindGroundObjects) false 0 "None"))
    (if (not _returnvalue_3)
      (bind (_outhit _returnvalue_4) (Collision|LineTraceForObjects _returnvalue (+ _returnvalue (* (Math|Vector|GetUpVector "0, 0, 0") (Variables|Default|GetFindGroundLength))) (Variables|Default|GetFindGroundObjects) false 0 "ForDuration"))
      (if _returnvalue_4
        (Transformation|SetActorLocation (.Location (Collision|BreakHitResult _outhit)) false false)
        (else
          (Default|Respawn (Variables|Default|GetRaceManager)))))))

(fn AddFallingtoVelocity
  (if (> (Variables|Default|GetVelocity) 5.0)
    (Variables|Default|SetVelocity (+ (Variables|Default|GetVelocity) (/ (Math|Float|Absolute(Float) (Variables|Default|GetFallingVelocity)) 2.0)))))