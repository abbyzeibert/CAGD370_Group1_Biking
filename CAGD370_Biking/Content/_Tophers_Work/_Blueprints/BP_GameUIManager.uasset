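; BP_GameUIManager spawns a configurable UI widget when play begins, for either in-game or menu-style screens.
; It casts player controller 0 to BP_PlayerController, creates the widget, passes it the race manager reference and adds it to the viewport.
; When IsGameUI is false, it switches to UI-only input focused on the widget and shows the mouse cursor.
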(event EventBeginPlay
  (bind _asbp_player_controller (Utilities|Casting|CastToBP_PlayerController (Game|GetPlayerController 0))
    (:then
      (bind _returnvalue (UserInterface|CreateWidget (Variables|Default|GetClass)))
      (Variables|/Game/_Tophers_Work/_Blueprints/WBP_GameUI.WBP_GameUI_C|SetBP_RaceManager _returnvalue (Variables|Default|GetBP%20Race%20Manager))
      (UserInterface|Viewport|AddtoViewport _returnvalue 0)
      (if (not (Variables|Default|GetIs_Game_UI))
        (Input|SetInputModeUIOnly _asbp_player_controller _returnvalue "DoNotLock" false)
        (Variables|/Script/Engine.PlayerController|SetbShowMouseCursor _asbp_player_controller true)))
    (:CastFailed
      (Development|PrintString "Cast Failed"))))

(fn ConstructionScript)