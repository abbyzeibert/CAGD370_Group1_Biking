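; Player bike for a race, driven by Enhanced Input and active between StartRace and EndRace.
; Tick runs custom kinematic movement from pedaling, friction, braking, steering and slope-based speed.
; A line trace snaps and tilts it to the ground or triggers manual falling, with jumps setting upward velocity.
; A capsule trace handles wall bounces and glancing deflections, while the spring arm camera follows slope and falls.
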(event Custom|StartRace
  (Variables|Default|SetIsActive true)
  (Development|PrintString "Race Started!"))

(event Custom|EndRace
  (Variables|Default|SetIsActive false)
  (Development|PrintString "Race Ended!"))

(event Input|EnhancedActionEvents|EnhancedInputActionIA_Pedal
  (params (ActionValue :type Boolean) (ElapsedSeconds :type Float%20%28double-precision%29) (TriggeredSeconds :type Float%20%28double-precision%29) (InputAction :type Input%20Action%20Object%20Reference :default "/Game/_Abbys_Work/Blueprints/Input/IA_Pedal.IA_Pedal"))
  (:Triggered
    ;[0 1 0 0.5] When player presses forward, adds to Velocity until max is reached
    (Variables|Default|SetIsPedaling true))
  (:Completed
    (Variables|Default|SetIsPedaling false)))

(event Input|EnhancedActionEvents|EnhancedInputActionIA_Brake
  (params (ActionValue :type Boolean) (ElapsedSeconds :type Float%20%28double-precision%29) (TriggeredSeconds :type Float%20%28double-precision%29) (InputAction :type Input%20Action%20Object%20Reference :default "/Game/_Abbys_Work/Blueprints/Input/IA_Brake.IA_Brake"))
  (:Triggered
    ;[0 1 0 0.5] Increases friction while braking
    (Variables|Default|SetFriction (Variables|Default|GetBrakingFriction))
    (Variables|Default|SetIsBraking true))
  (:Completed
    (Variables|Default|SetFriction (Variables|Default|GetStandardFriction))
    (Variables|Default|SetIsBraking false)))

(event Input|EnhancedActionEvents|EnhancedInputActionIA_Turn
  (params (ActionValue :type Float%20%28double-precision%29) (ElapsedSeconds :type Float%20%28double-precision%29) (TriggeredSeconds :type Float%20%28double-precision%29) (InputAction :type Input%20Action%20Object%20Reference :default "/Game/_Abbys_Work/Blueprints/Input/IA_Turn.IA_Turn"))
  (:Triggered
    ;[0 1 0 0.5] Activates & deactivates turning
    (if (Variables|Default|GetOnGround)
      (Variables|Default|SetTurnDir ActionValue)
      (else
        (Variables|Default|SetTurnDir 0.0 :!label _label))))
  (:Completed
    (goto _label)))

(event Input|EnhancedActionEvents|EnhancedInputActionIA_Jump
  (params (ActionValue :type Boolean) (ElapsedSeconds :type Float%20%28double-precision%29) (TriggeredSeconds :type Float%20%28double-precision%29) (InputAction :type Input%20Action%20Object%20Reference :default "/Game/_Abbys_Work/Blueprints/Input/IA_Jump.IA_Jump"))
  (if (Variables|Default|GetIsActive)
    (CallFunction|Jump)))

(event EventBeginPlay
  (bind _returnvalue (Game|GetPlayerController 0))
  (Utilities|FlowControl|Delay 0.1)
  ;[0 1 0 0.5] Setting up input mapping
  (bind _asbp_player_controller (Utilities|Casting|CastToBP_PlayerController _returnvalue))
  (Input|AddMappingContext (PlayerController|LocalPlayerSubsystems|GetEnhancedInputLocalPlayerSubsystem _asbp_player_controller) "/Game/_Abbys_Work/Blueprints/Input/IMC_BikeControls.IMC_BikeControls" 0 "(bIgnoreAllPressedKeysUntilRelease=True,bForceImmediately=False,bNotifyUserSettings=False)")
  (Input|SetInputModeGameOnly _returnvalue false)
  (bind _returnvalue_2 (Actor|GetActorOfClass "/Game/_Abbys_Work/Blueprints/BP_RaceManager.BP_RaceManager_C"))
  (Variables|Default|SetRaceManager _returnvalue_2))

(event Collision|EventActorBeginOverlap
  (params (OtherActor :type Actor%20Object%20Reference)))

(event EventTick
  (params (DeltaSeconds :type Float%20%28single-precision%29))
  (bind _returnvalue (Transformation|GetActorForwardVector))
  (bind _returnvalue_2 (Math|Trig|Sin(Degrees) (.z _returnvalue)))
  (bind _output_get (Variables|Default|SetDelta%20Seconds DeltaSeconds))
  (if (Variables|Default|GetIsActive)
    (if (Variables|Default|GetOnGround)
      (if (Variables|Default|GetIsPedaling)
        (Variables|Default|SetVelocity (Math|Float|Clamp(Float) (+ (* (Variables|Default|GetAcceleration) (Variables|Default|GetDelta%20Seconds)) (Math|Float|Clamp(Float) (- (Variables|Default|GetVelocity) (* (Variables|Default|GetFriction) (Variables|Default|GetDelta%20Seconds))) 0.0 (Variables|Default|GetMaxVelocity))) -1e+02 (Variables|Default|GetMaxVelocity)))
        (else
          (Variables|Default|SetVelocity (Math|Float|Clamp(Float) (- (Variables|Default|GetVelocity) (* (Variables|Default|GetFriction) (Variables|Default|GetDelta%20Seconds))) 0.0 (Variables|Default|GetMaxVelocity))))))
    ;[0 1 0 0.5] Angles bike based on slope and changes velocity from slope
    (CallFunction|TurnAlongSlope)
    (Variables|Default|SetBikeAngle _returnvalue_2)
    ;[0 1 0 0.5] Moves bike in forward direction with given velocity
    (Variables|Default|SetVelocity (- (Variables|Default|GetVelocity) (* _returnvalue_2 (Variables|Default|GetHillSpeedMultiplier) (Variables|Default|GetDelta%20Seconds))))
    (Transformation|AddActorWorldOffset (* (Transformation|GetActorForwardVector) (Variables|Default|GetVelocity) _output_get))
    ;[0 1 0 0.5] Turns bike based on turn direction and speed
    (Class|Actor|AddActorWorldRotation (Math|Rotator|MakeRotator 0.0 0.0 (* (Variables|Default|GetTurnDir) (Variables|Default|GetTurnSpeed) (Variables|Default|GetDelta%20Seconds))))
    (CallFunction|BounceOffWalls)
    (CallFunction|AngleCameratoSlope)))

(fn ConstructionScript)

(fn TurnAlongSlope
  (bind _returnvalue (Transformation|GetActorLocation))
  (bind _returnvalue_2 (Transformation|GetActorLocation))
  (bind (_outhit _returnvalue_3) (Collision|LineTraceForObjects _returnvalue_2 (+ _returnvalue_2 (* (Math|Vector|GetUpVector "0, 0, 0") (Variables|Default|GetDownCastLength))) (Variables|Default|GetObject%20Types) false 0 "None"))
  (if _returnvalue_3
    (Variables|Default|SetOnGround true)
    (Variables|Default|SetDownCastLength -5e+01)
    (Variables|Default|SetFallingVelocity 0.0)
    (Transformation|SetActorLocation (Math|Vector|MakeVector (.x _returnvalue) (.y _returnvalue) (+ (Variables|Default|GetBikeHeight) (.z (.ImpactPoint (Collision|BreakHitResult _outhit))))) false false)
    (Transformation|SetActorRotation (Math|Rotator|MakeRotator (.roll (Math|Rotator|MakeRotfromXZ (Transformation|GetActorForwardVector) (.ImpactNormal (Collision|BreakHitResult _outhit)))) (.pitch (Class|KismetMathLibrary|MakeRotfromYZ (Transformation|GetActorRightVector) (.ImpactNormal (Collision|BreakHitResult _outhit)))) (.yaw (Transformation|GetActorRotation))))
    (else
      (if (Variables|Default|GetOnGround)
        (Variables|Default|SetOnGround false)
        (Variables|Default|SetFallingVelocity 0.0)
        (Variables|Default|SetDownCastLength -3e+01))
      (CallFunction|Fall)))
  (return))

(fn Jump
  (Transformation|AddActorWorldOffset (Math|Vector|MakeVector 0.0 0.0 1e+01))
  (Variables|Default|SetOnGround false)
  (Variables|Default|SetDownCastLength -3e+01)
  (Variables|Default|SetFallingVelocity (Variables|Default|GetJumpForce))
  (Transformation|SetActorRotation (Math|Rotator|MakeRotator 0.0 0.0 (.yaw (Transformation|GetActorRotation)))))

(fn Fall
  (bind _delta_seconds (Variables|Default|GetDelta%20Seconds))
  (bind _output_get (Variables|Default|SetFallingVelocity (- (Variables|Default|GetFallingVelocity) (* (Variables|Default|GetGravity) _delta_seconds))))
  (Transformation|AddActorLocalOffset (Math|Vector|MakeVector 0.0 0.0 (* _output_get _delta_seconds)) false false))

(fn AngleCameratoSlope
  (bind _returnvalue (Transformation|GetActorRotation))
  (bind _springarm (Variables|Default|GetSpringArm))
  (bind _springarm_2 (Variables|Default|GetSpringArm))
  (bind _fallingacceleration (LocalVariables|GetFallingAcceleration))
  (bind _delta_seconds (Variables|Default|GetDelta%20Seconds))
  (bind _fallingvelocity (Variables|Default|GetFallingVelocity))
  (bind _defaultspringspeed (Variables|Default|GetDefaultSpringSpeed))
  (bind _returnvalue_2 (Class|SpringArmComponent|GetTargetRotation _springarm_2))
  (bind _returnvalue_3 (* _fallingacceleration _delta_seconds -1.0))
  (if (Variables|Default|GetOnGround)
    (Variables|/Script/Engine.SpringArmComponent|SetSocketOffset _springarm (Math|Vector|MakeVector (- (Variables|Default|GetDefaultSpringSpeed) (/ (Variables|Default|GetVelocity) 1e+01)) 0.0 (Math|Float|Lerp (.z (Variables|/Script/Engine.SpringArmComponent|GetSocketOffset _springarm)) (- (Variables|Default|GetDefaultSpringPos) (* (Variables|Default|GetBikeAngle) 7.5e+03)) 0.15)))
    (Transformation|SetWorldRotation (Variables|Default|GetSpringArm) (Math|Rotator|MakeRotator 0.0 (Math|Float|Clamp(Float) (+ (Variables|Default|GetDefaultCamRot) (* (Variables|Default|GetBikeAngle) 1875.0)) -2e+01 2e+01) (.yaw _returnvalue)) false false)
    (elif (> (.pitch _returnvalue_2) (LocalVariables|GetMaxFallingAngle))
      (Transformation|AddLocalRotation _springarm_2 (Math|Rotator|MakeRotator 0.0 _returnvalue_3 0.0) false false)
      (Transformation|SetWorldRotation _springarm_2 (Math|Rotator|MakeRotator 0.0 (.pitch _returnvalue_2) (.yaw _returnvalue)) false false)
      (Variables|/Script/Engine.SpringArmComponent|SetSocketOffset _springarm_2 (Math|Vector|MakeVector (Math|Float|Clamp(Float) (+ _fallingvelocity _defaultspringspeed) -6e+02 _defaultspringspeed) 0.0 (Math|Float|Clamp(Float) (- (.z (Variables|/Script/Engine.SpringArmComponent|GetSocketOffset _springarm_2)) (/ _fallingvelocity 2e+01)) (.z (Variables|/Script/Engine.SpringArmComponent|GetSocketOffset _springarm_2)) 1e+03)))
      (else
        (Transformation|AddWorldRotation _springarm_2 (Math|Rotator|MakeRotator 0.0 _returnvalue_3 0.0) false false)))))

(fn BounceOffWalls
  (bind _returnvalue (Transformation|GetActorForwardVector))
  (bind _returnvalue_2 (Transformation|GetActorForwardVector))
  (bind _returnvalue_3 (Transformation|GetActorLocation))
  (bind _returnvalue_4 (* _returnvalue_2 5e+01))
  (bind (_outhit _returnvalue_5) (Class|KismetSystemLibrary|CapsuleTraceSingleforObjects (+ _returnvalue_4 _returnvalue_3) (- _returnvalue_3 _returnvalue_4) 5.0 0.0 (Variables|Default|GetObject%20Types) false 0 "ForDuration" true))
  (if _returnvalue_5
    (if (> (Variables|Default|GetVelocity) 3e+02)
      (if (and (<= (* (Math|Trig|Sin(Degrees) (.Z (Math|Vector|BreakVector (.ImpactNormal (Collision|BreakHitResult _outhit))))) 1e+02) 1.0) (>= (* (Math|Trig|Sin(Degrees) (.Z (Math|Vector|BreakVector (.ImpactNormal (Collision|BreakHitResult _outhit))))) 1e+02) -1.0))
        (if (> (Math|Float|Absolute(Float) (Class|KismetMathLibrary|VectorCosineAngle2D (.ImpactNormal (Collision|BreakHitResult _outhit)) _returnvalue)) 0.85)
          (Transformation|AddActorWorldOffset (* (.ImpactNormal (Collision|BreakHitResult _outhit)) 2e+01))
          (CallFunction|Jump)
          (Variables|Default|SetVelocity -3e+02)
          (else
            (Transformation|SetActorRotation (Math|Conversions|RotationFromXVector (Math|Vector|GetReflectionVector _returnvalue (.ImpactNormal (Collision|BreakHitResult _outhit)))))
            (Transformation|AddActorWorldOffset (* (.ImpactNormal (Collision|BreakHitResult _outhit)) 2e+01))
            (Variables|Default|SetVelocity (* (Variables|Default|GetVelocity) (- 1.0 (Math|Float|Absolute(Float) (Class|KismetMathLibrary|VectorCosineAngle2D (.ImpactNormal (Collision|BreakHitResult _outhit)) _returnvalue)))))
            (Development|PrintString "Bonk!"))))
      (else
        (Variables|Default|SetVelocity 0.0)))))